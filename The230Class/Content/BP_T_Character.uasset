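; BP_T_Character is a character Blueprint that handles an area stun ability and opening the pause menu.
; The Stun input runs a multi-sphere object trace around the character and calls StunBegin on each BPT_PublicEnemy hit.
; A Timer counted down in Tick gates the stun with a ten-second cooldown.
; The E key clears all widgets, shows the PauseBP widget with the mouse cursor and pauses the game.
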(event EventBeginPlay)

(event Collision|EventActorBeginOverlap
  (params (OtherActor :type Actor%20Object%20Reference)))

(event EventTick
  (params (DeltaSeconds :type Float%20%28single-precision%29))
  (Variables|Default|SetTimer (- (Variables|Default|GetTimer) DeltaSeconds)))

(event Input|ActionEvents|InputActionStun
  (params (Key :type Key%20Structure :default "None"))
  (bind _returnvalue (Transformation|GetActorLocation))
  (:Pressed
    (if (<= (Variables|Default|GetTimer) 0.0)
      (Variables|Default|SetTimer 1e+01)
      (bind (_outhits _returnvalue_2) (Collision|MultiSphereTraceForObjects _returnvalue _returnvalue (Variables|Default|GetStunRadius) (Variables|Default|GetStunObjectTypes) false 0 "None"))
      (if _returnvalue_2
        (for _array_element _outhits
          (bind _asbpt_public_enemy (Utilities|Casting|CastToBPT_PublicEnemy (.hitactor _array_element)))
          (Default|StunBegin _asbpt_public_enemy))))))

(event Input|KeyboardEvents|E
  (params (Key :type Key%20Structure :default "None"))
  (:Pressed
    (Viewport|RemoveAllWidgets)
    (bind _returnvalue (UserInterface|CreateWidget "/Game/PauseBP.PauseBP_C"))
    (UserInterface|Viewport|AddtoViewport _returnvalue 0)
    (Variables|/Script/Engine.PlayerController|SetbShowMouseCursor (Game|GetPlayerController 0) true)
    (Game|SetGamePaused true)))

(fn ConstructionScript)