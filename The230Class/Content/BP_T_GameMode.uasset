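; Game mode that manages level flow, screen widgets and music for gameplay.
; BeginPlay shows the HUD and calls PlaySong, which plays music and applies saved volumes only when a Settings save exists.
; Tick polls character health and calls LoseUI every frame at zero or below.
; Helper functions swap win, lose and menu widgets, resume from pause, restart, or advance through the Levels array with main-menu fallback.
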(event EventBeginPlay
  (bind _returnvalue (UserInterface|CreateWidget "/Game/GameHUD.GameHUD_C"))
  (UserInterface|Viewport|AddtoViewport _returnvalue 0)
  (Variables|/Script/Engine.PlayerController|SetbShowMouseCursor (Game|GetPlayerController 0) false)
  (CallFunction|PlaySong))

(event EventTick
  (params (DeltaSeconds :type Float%20%28single-precision%29))
  (bind _asbp_t_character (Utilities|Casting|CastToBP_T_Character (Game|Player|GetPlayerPawn 0)))
  (if (<= (Variables|/Script/The230Class.T_Character|GetCurrentHealth _asbp_t_character) 0.0)
    (CallFunction|LoseUI)))

(fn ConstructionScript)

(fn RestartLevel
  (bind _returnvalue (Game|GetCurrentLevelName true))
  (Game|OpenLevel(byName) (Utilities|String|StringToName _returnvalue))
  (return))

(fn MainMenu
  (Game|OpenLevel(byObjectReference) "/Game/Untitled.Untitled")
  (return))

(fn NextLevel
  (for _index (range 1 (Utilities|Array|LastIndex (Variables|Default|GetLevels)))
    (Variables|Default|SetLevelIndex 0)
    (bind _returnvalue (Game|GetCurrentLevelName true))
    (if (Utilities|Enum|Equal(Enum) _returnvalue (Utilities|GetObjectName (Utilities|ResolveSoftReference (Utilities|Array|Get(acopy) (Variables|Default|GetLevels) (- (Variables|Default|GetLevelIndex) 1)))))
      (Game|OpenLevel(byObjectReference) (Utilities|Array|Get(acopy) (Variables|Default|GetLevels) (Variables|Default|GetLevelIndex)))
      (return)))
  (CallFunction|MainMenu)
  (return))

(fn WinUI
  (Viewport|RemoveAllWidgets)
  (bind _returnvalue (UserInterface|CreateWidget "/Game/WinWidgetBP.WinWidgetBP_C"))
  (UserInterface|Viewport|AddtoViewport _returnvalue 0)
  (Variables|/Script/Engine.PlayerController|SetbShowMouseCursor (Game|GetPlayerController 0) true))

(fn LoseUI
  (Viewport|RemoveAllWidgets)
  (bind _returnvalue (UserInterface|CreateWidget "/Game/GameOverWidgetBP.GameOverWidgetBP_C"))
  (UserInterface|Viewport|AddtoViewport _returnvalue 0)
  (Variables|/Script/Engine.PlayerController|SetbShowMouseCursor (Game|GetPlayerController 0) true))

(fn MMUI
  (Viewport|RemoveAllWidgets)
  (bind _returnvalue (UserInterface|CreateWidget "/Game/MAINMenuBP.MAINMenuBP_C"))
  (UserInterface|Viewport|AddtoViewport _returnvalue 0)
  (Variables|/Script/Engine.PlayerController|SetbShowMouseCursor (Game|GetPlayerController 0) true))

(fn Resume
  (Viewport|RemoveAllWidgets)
  (bind _returnvalue (UserInterface|CreateWidget "/Game/GameHUD.GameHUD_C"))
  (UserInterface|Viewport|AddtoViewport _returnvalue 0)
  (Variables|/Script/Engine.PlayerController|SetbShowMouseCursor (Game|GetPlayerController 0) false)
  (Game|SetGamePaused false))

(fn PlaySong
  (Audio|PushSoundMixModifier "/Game/Sound/MasterSound.MasterSound")
  (bind _returnvalue (SaveGame|DoesSaveGameExist "Settings"))
  (if _returnvalue
    (Class|GameplayStatics|SetBaseSoundMix "/Game/Sound/MasterSound.MasterSound")
    (Audio|PlaySound2D "/Game/sweet-life-luxury-chill-438146.sweet-life-luxury-chill-438146" 1.0 1.0 0.0 0 0)
    (bind _returnvalue_2 (SaveGame|LoadGamefromSlot "Settings"))
    (bind _assame_game_bp (Utilities|Casting|CastToSameGameBP _returnvalue_2))
    (bind _output_get (Variables|Default|SetAs%20Same%20Game%20BP _assame_game_bp))
    (Audio|SetSoundMixClassOverride "/Game/Sound/MasterSound.MasterSound" "/Game/Sound/MasterFXSoound.MasterFXSoound" (Variables|/Game/SaveGame/SameGameBP.SameGameBP_C|GetSFXVol _output_get) 1.0 1.0 true)
    (Audio|SetSoundMixClassOverride "/Game/Sound/MasterSound.MasterSound" "/Game/Sound/MUSCISOmd.MUSCISOmd" (Variables|/Game/SaveGame/SameGameBP.SameGameBP_C|GetSongVol _output_get) 1.0 1.0 true)))